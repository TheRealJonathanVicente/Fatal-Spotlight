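; Dialogue component that runs branching, data-table-driven conversations with a named character, tracking that character's frustration.
; Interact opens or advances the dialogue widget, following each row's next row and table, or closes it and calls ReduceTime on the game mode.
; Open-ended rows spawn option widgets whose picks load new rows, or the "Frustration" row once the frustration limit is reached.
; TransitionDay swaps in that day's table and resets progress and frustration.
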(event Custom|OptionSelected
  (params (RowName :type Name) (DataTable :type Data%20Table%20Object%20Reference))
  ;[0.06774 0.15 0.06339 0.5] Check frustration and if clue before updating dialogue
  (if (>= (Variables|Default|GetFrustrationAmount) 6)
    (Development|PrintString "Frustration exceeded")
    (bind _returnvalue (Utilities|GetDataTableRow DataTable "Frustration")
      (:then
        (CallFunction|WritetoScreen _returnvalue)))
    (else
      (bind _returnvalue_2 (Utilities|GetDataTableRow DataTable RowName)
        (:then
          (CallFunction|WritetoScreen _returnvalue_2))))))

(event Custom|Create%20Widget
  (params (Option :type Options%20Dialogue%20Structure%20Structure))
  (bind (_optionname _row _datatable _isleave _isclue _cluetext _frustration) (Utilities|Struct|BreakOptionsDialogue_Structure Option))
  ;[0.000129 0.15 0.1422 0.5] Options Widget Creation
  (bind _returnvalue (UserInterface|CreateWidget "/Game/Scripts/Dialogue/WB_Options.WB_Options_C" 0 (Utilities|Text|ToText(Name) _optionname) self _row _datatable _isleave _frustration _isclue _cluetext (Variables|Default|GetDialogueWidget) (Variables|Default|GetCharacterNum)))
  (Widget|Panel|AddChild (Variables|/Game/Scripts/Dialogue/WB_Dialogue.WB_Dialogue_C|GetOptionScrollBox (Variables|Default|GetDialogueWidget)) _returnvalue))

(event Custom|write%20to%20screen
  (params (NewParam :type Dialogue%20Sructure%20Structure))
  (bind (_dialogue _row _datatable _enddialogue_ _openendeddialogue_ _openendeddialogueoptions) (Utilities|Struct|BreakDialogue_Sructure NewParam))
  (bind _returnvalue (Game|GetPlayerController 0))
  ;[0.1452 0.15 0.1487 0.5] Dialogue updating
  (Widget|Panel|ClearChildren (Variables|/Game/Scripts/Dialogue/WB_Dialogue.WB_Dialogue_C|GetOptionScrollBox (Variables|Default|GetDialogueWidget)))
  (Default|UpdateDialogue (Variables|Default|GetDialogueWidget) _dialogue)
  (Variables|Default|SetRow%20Name _row)
  (Variables|Default|SetData%20Table _datatable)
  (Variables|Default|SetEndDialogue _enddialogue_)
  (Input|SetInputModeGameandUI _returnvalue 0 "DoNotLock" true false)
  (Variables|/Script/Engine.PlayerController|SetbShowMouseCursor _returnvalue true)
  (if _openendeddialogue_
    (for _array_element _openendeddialogueoptions
      (CallFunction|CreateWidget _array_element))))

(event EventBeginPlay)

(event EventTick
  (params (DeltaSeconds :type Float%20%28single-precision%29)))

(event EventInteract
  (params (playerref :type BP%20Detective%20Object%20Reference) (Journal :type W%20Journal%20Object%20Reference))
  (bind _returnvalue (Game|GetPlayerController 0))
  ;[0.03538 0.02536 0.15 0.5] Initial Chat Box Setup
  (if (Variables|Default|GetEndDialogue)
    (CallFunction|LeaveDialogue)
    (else
      (Utilities|IsValid (Variables|Default|GetDialogueWidget)
        (:Is%20Valid
          (bind _returnvalue_2 (Utilities|GetDataTableRow (Variables|Default|GetData%20Table) (Variables|Default|GetRow%20Name))
            (:then
              (Default|UpdateDialogue (Variables|Default|GetDialogueWidget) (.Dialogue (Utilities|Struct|BreakDialogue_Sructure _returnvalue_2)))
              (Variables|Default|SetRow%20Name (.Row (Utilities|Struct|BreakDialogue_Sructure _returnvalue_2)))
              (Variables|Default|SetData%20Table (.DataTable (Utilities|Struct|BreakDialogue_Sructure _returnvalue_2)))
              (Variables|Default|SetEndDialogue (.EndDialogue? (Utilities|Struct|BreakDialogue_Sructure _returnvalue_2))))))
        (:Is%20Not%20Valid
          (bind _returnvalue_3 (Utilities|GetDataTableRow (Variables|Default|GetData%20Table) (Variables|Default|GetRow%20Name))
            (:then
              (bind _returnvalue_4 (UserInterface|CreateWidget "/Game/Scripts/Dialogue/WB_Dialogue.WB_Dialogue_C" 0 (Utilities|Text|ToText(Name) (Variables|Default|GetName)) (.Dialogue (Utilities|Struct|BreakDialogue_Sructure _returnvalue_3))))
              (bind _output_get (Variables|Default|SetDialogueWidget _returnvalue_4))
              (UserInterface|Viewport|AddtoViewport _output_get 0)
              (Progress|SetPercent (Variables|/Game/Scripts/Dialogue/WB_Dialogue.WB_Dialogue_C|GetProgressBar_0 (Variables|Default|GetDialogueWidget)) (/ (Math|Conversions|ToFloat(Integer) (Variables|Default|GetFrustrationAmount)) 6.0))
              (Variables|Default|SetRow%20Name (.Row (Utilities|Struct|BreakDialogue_Sructure _returnvalue_3)))
              (Variables|Default|SetData%20Table (.DataTable (Utilities|Struct|BreakDialogue_Sructure _returnvalue_3)))
              (Variables|Default|SetEndDialogue (.EndDialogue? (Utilities|Struct|BreakDialogue_Sructure _returnvalue_3)))
              (Input|SetInputModeGameandUI _returnvalue 0 "DoNotLock" true false)
              (Variables|/Script/Engine.PlayerController|SetbShowMouseCursor _returnvalue true)
              (if (.OpenEndedDialogue? (Utilities|Struct|BreakDialogue_Sructure _returnvalue_3))
                (for _array_element (.OpenEndedDialogueOptions (Utilities|Struct|BreakDialogue_Sructure _returnvalue_3))
                  (CallFunction|CreateWidget _array_element))))))))))

(event EventLeaveDialogue
  (bind _returnvalue (Game|GetPlayerController 0))
  ;[0.15 0.0316 0.03482 0.5] Leaving Dialogue
  (Utilities|IsValid (Variables|Default|GetDialogueWidget)
    (:Is%20Valid
      (Widget|RemovefromParent (Variables|Default|GetDialogueWidget))
      (Variables|Default|SetEndDialogue false)
      (Variables|Default|SetDialogueWidget 0)
      (Input|SetInputModeGameandUI _returnvalue 0 "DoNotLock" true false)
      (Variables|/Script/Engine.PlayerController|SetbShowMouseCursor _returnvalue false)
      (Input|SetInputModeGameOnly _returnvalue false)
      (bind _returnvalue_2 (Actor|GetActorOfClass "/Game/Scripts/Player_Controller/BP_GameMode.BP_GameMode_C"))
      (Default|ReduceTime _returnvalue_2 5))))

(event EventManageFrustration
  (params (Frustration :type Integer))
  ;[0.15 0.15 0.15 0.5] Frustration Management
  (bind _output_get (Variables|Default|SetFrustrationAmount (+ Frustration (Variables|Default|GetFrustrationAmount))))
  (Progress|SetPercent (Variables|/Game/Scripts/Dialogue/WB_Dialogue.WB_Dialogue_C|GetProgressBar_0 (Variables|Default|GetDialogueWidget)) (/ (Math|Conversions|ToFloat(Integer) _output_get) 6.0)))

(event EventTransitionDay
  (params (DayNum :type Integer))
  ;[0.15 0.1124 0.03045 0.5] DataTable Reassignment
  (Variables|Default|SetData%20Table (Utilities|Array|Get(acopy) (Variables|Default|GetLaterDataTables) DayNum))
  (Variables|Default|SetRow%20Name "1")
  (Variables|Default|SetEndDialogue false)
  (Variables|Default|SetFrustrationAmount 0))
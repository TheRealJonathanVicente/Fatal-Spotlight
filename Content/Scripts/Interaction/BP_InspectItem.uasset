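; Inspection actor that displays an examined item with a name and description widget while taking input from the character.
; Mouse drag or gamepad stick rotates the mesh.
; Tick compares its forward vector to a target rotation via dot product; holding alignment for one second adds an extra clue detail to the journal with a sound.
; Interact reduces game-mode time, restores character input and destroys the actor.
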(event Custom|Set%20Inspect%20Rotation
  (params (ItemRotation :type Rotator))
  (bind _item (Variables|Default|GetItem))
  (bind _returnvalue (Transformation|GetWorldTransform _item))
  ;[0.15 0.15 0.15 0.5] Rotation setting
  (bind _output_get (Variables|Default|SetItem%20Rotation ItemRotation))
  (Transformation|SetWorldTransform _item (Math|Transform|MakeTransform (.location _returnvalue) _output_get (.scale _returnvalue)) false false))

(event Custom|Set%20Inspect%20Scale
  (params (Inspection%20Scale :type Vector))
  (bind _item (Variables|Default|GetItem))
  (bind _returnvalue (Transformation|GetWorldTransform _item))
  ;[0.15 0.15 0.15 0.5] Rotation setting
  (Transformation|SetWorldTransform _item (Math|Transform|MakeTransform (.location _returnvalue) (.rotation _returnvalue) Inspection%20Scale) false false))

(event Custom|Detail%20found
  (Default|AddDetails (Variables|Default|GetJournal%20Ref) (Variables|Default|GetClueNum) (Variables|Default|GetExtrDetails))
  (Audio|PlaySound2D "/Game/Sound/SX_ClueDiscoery.SX_ClueDiscoery" 1.0 1.0 0.0 0 0)
  (Variables|Default|SetDetailFound true))

(event Input|EnhancedActionEvents|EnhancedInputActionIA_Interact
  (params (ActionValue :type Boolean) (ElapsedSeconds :type Float%20%28double-precision%29) (TriggeredSeconds :type Float%20%28double-precision%29) (InputAction :type Input%20Action%20Object%20Reference :default "/Game/Scripts/Player_Controller/IO/IA_Interact.IA_Interact"))
  (bind _returnvalue (Game|GetPlayerController 0))
  ;[0.15 0.15 0.15 0.5] Initialization and leaving
  (:Started
    (bind _returnvalue_2 (Actor|GetActorOfClass "/Game/Scripts/Player_Controller/BP_GameMode.BP_GameMode_C"))
    (Default|ReduceTime _returnvalue_2 (stale EventInspect ReductionAmount))
    (Input|DisableInput _returnvalue)
    (Input|EnableInput (stale EventInspect _output_get) _returnvalue)
    (Utilities|IsValid (Variables|Default|GetWidget)
      (:Is%20Valid
        (Widget|RemovefromParent (Variables|Default|GetWidget))
        (Variables|Default|SetWidget 0)
        (Actor|DestroyActor)))))

(event EventTick
  (params (DeltaSeconds :type Float%20%28single-precision%29))
  (if (Math|Float|InRange(Float) (Math|Vector|DotProduct (Math|Vector|GetForwardVector (Transformation|GetWorldRotation (Variables|Default|GetItem))) (Math|Vector|GetForwardVector (Variables|Default|GetExtraDetailRotation))) 0.8 1.0)
    (if (Variables|Default|GetSearchForDetail?)
      (if (not (Variables|Default|GetDetailFound))
        (bind _returnvalue (Utilities|Time|SetTimerbyEvent (delegate Custom|Detail%20found) 1.0))
        (Variables|Default|SetSearchForDetail? false)))
    (else
      (Utilities|Time|ClearandInvalidateTimerbyHandle _returnvalue)
      (Variables|Default|SetSearchForDetail? true))))

(event EventInspect
  (params (Character :type BP%20Detective%20Object%20Reference) (InspectedItem :type Static%20Mesh%20Object%20Reference) (JournalRef :type W%20Journal%20Object%20Reference) (ItemName :type Text) (Item%20Description :type Text) (ExtraDetails :type Text) (ClueNum :type Integer) (ExtraDetailRotation :type Rotator :default "0, 0, 0") (ReductionAmount :type Integer))
  (bind _returnvalue (Game|GetPlayerController 0))
  ;[0.15 0.15 0.15 0.5] Initialization and leaving
  (Variables|Default|SetExtraDetailRotation ExtraDetailRotation)
  (Variables|Default|SetExtrDetails ExtraDetails)
  (Variables|Default|SetClueNum ClueNum)
  (Variables|Default|SetJournal%20Ref JournalRef)
  (bind _output_get (Variables|Default|SetCharacter Character))
  (Components|StaticMesh|SetStaticMesh (Variables|Default|GetItem) InspectedItem)
  (bind _returnvalue_2 (UserInterface|CreateWidget "/Game/Scripts/Interaction/W_Inspect.W_Inspect_C" 0 ItemName Item%20Description))
  (bind _output_get_2 (Variables|Default|SetWidget _returnvalue_2))
  (UserInterface|Viewport|AddtoViewport _output_get_2 0)
  (Input|DisableInput _output_get _returnvalue)
  (Input|EnableInput _returnvalue))

(event Input|MouseEvents|MouseX
  (params (AxisValue :type Float%20%28single-precision%29))
  ;[0.15 0.15 0.15 0.5] Controls
  (if (Variables|Default|GetRotate?)
    (Transformation|SetWorldRotation (Variables|Default|GetItem) (Math|Rotator|CombineRotators (Transformation|GetWorldRotation (Variables|Default|GetItem)) (Math|Rotator|MakeRotator 0.0 0.0 (* AxisValue -3.0))) false false)))

(event Input|MouseEvents|MouseY
  (params (AxisValue :type Float%20%28single-precision%29))
  ;[0.15 0.15 0.15 0.5] Controls
  (if (Variables|Default|GetRotate?)
    (Transformation|SetWorldRotation (Variables|Default|GetItem) (Math|Rotator|CombineRotators (Transformation|GetWorldRotation (Variables|Default|GetItem)) (Math|Rotator|MakeRotator 0.0 (* AxisValue -3.0) 0.0)) false false)))

(event Input|GamepadEvents|GamepadRightX
  (params (AxisValue :type Float%20%28single-precision%29))
  ;[0.15 0.15 0.15 0.5] Controls
  (Transformation|SetWorldRotation (Variables|Default|GetItem) (Math|Rotator|CombineRotators (Transformation|GetWorldRotation (Variables|Default|GetItem)) (Math|Rotator|MakeRotator 0.0 0.0 (* AxisValue -3.0))) false false))

(event Input|GamepadEvents|GamepadRightY
  (params (AxisValue :type Float%20%28single-precision%29))
  ;[0.15 0.15 0.15 0.5] Controls
  (Transformation|SetWorldRotation (Variables|Default|GetItem) (Math|Rotator|CombineRotators (Transformation|GetWorldRotation (Variables|Default|GetItem)) (Math|Rotator|MakeRotator 0.0 (* AxisValue -3.0) 0.0)) false false))

(event Input|MouseEvents|LeftMouseButton
  (params (Key :type Key%20Structure))
  ;[0.15 0.15 0.15 0.5] Controls
  (:Pressed
    (Variables|Default|SetRotate? true))
  (:Released
    (Variables|Default|SetRotate? false)))

(fn ConstructionScript)
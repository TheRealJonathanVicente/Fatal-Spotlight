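; BP_LockedDoor is a puzzle door that opens once enough items have been collected.
; CollectItem increments a counter, and overlapping the box trigger compares it against the required maximum.
; When the count is met, OpenDoor plays a timeline that lerps the hinge's yaw to swing the door open.
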(event OnComponentBeginOverlap(Box)
  (params (OverlappedComponent :type Primitive%20Component%20Object%20Reference) (OtherActor :type Actor%20Object%20Reference) (OtherComp :type Primitive%20Component%20Object%20Reference) (OtherBodyIndex :type Integer) (bFromSweep :type Boolean) (SweepResult :type Hit%20Result%20Structure%20%28by%20ref%29))
  (if (>= (Variables|Default|GetCurrent%20Items%20Collected) (Variables|Default|GetMax%20Items%20Collected))
    (CallFunction|OpenDoor)))

(event Custom|OpenDoor
  (bind _door_rotation (Timeline|OpenDoorAnimation Play)
    (:Update
      (Transformation|SetRelativeRotation (Variables|Default|GetHindge) (Math|Rotator|MakeRotator 0.0 0.0 (Math|Float|Lerp 0.0 1.2e+02 _door_rotation)) false false))))

(event Custom|CollectItem
  (Math|Integer|IncrementInt (Variables|Default|GetCurrent%20Items%20Collected)))

(fn ConstructionScript)
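; BP_GameMode is a game mode that tracks the time left in the day and handles the end-of-day transition.
; ReduceTime subtracts a set amount from the remaining time, or triggers TransitionDay when that would reach zero or below.
; TransitionDay teleports every BP_NPC to a transform from NPCLocations, paired by array index.
; It does not reset the remaining time, and BeginPlay and Tick are empty.
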(event Custom|Transition%20Day
  ;[0.15 0.15 0.15 0.5] End of day npc movement
  (bind _outactors (Actor|GetAllActorsOfClass "/Game/Scripts/Dialogue/BP_NPC.BP_NPC_C"))
  (for _array_element _outactors
    (Transformation|SetActorTransform _array_element (Utilities|Array|Get(acopy) (Variables|Default|GetNPC%20locations) (Variables|Default|GetArray%20index)) false true)
    (Variables|Default|SetArray%20index (+ (Variables|Default|GetArray%20index) 1))))

(event EventBeginPlay)

(event EventTick
  (params (DeltaSeconds :type Float%20%28single-precision%29)))

(event EventReduceTime
  (params (TimeReducing? :type Boolean))
  (if (<= (- (Variables|Default|GetTimeRemaining) (Variables|Default|GetReduceTimeAmount)) 0)
    (Development|PrintString "Day over!")
    (CallFunction|TransitionDay)
    (else
      (Variables|Default|SetTimeRemaining (- (Variables|Default|GetTimeRemaining) (Variables|Default|GetReduceTimeAmount)))
      (Development|PrintString "Time Reduced"))))

(fn ConstructionScript)
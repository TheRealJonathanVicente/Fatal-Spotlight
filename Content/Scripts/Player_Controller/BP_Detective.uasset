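; BP_Detective is the player character, handling Enhanced Input movement, look, jump, NPC dialogue and a clue journal.
; A sphere overlap stores an interface-implementing actor for the interact key and notifies it on exit.
; It spawns a hidden journal widget, forwards clue updates to it, and toggles it with movement and cursor changes.
; Velocity starts or stops a footstep timeline, but the wood-sound handler is marked as never run.
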(event OnComponentBeginOverlap(Sphere)
  (params (OverlappedComponent :type Primitive%20Component%20Object%20Reference) (OtherActor :type Actor%20Object%20Reference) (OtherComp :type Primitive%20Component%20Object%20Reference) (OtherBodyIndex :type Integer) (bFromSweep :type Boolean) (SweepResult :type Hit%20Result%20Structure%20%28by%20ref%29))
  ;[0.15 0.15 0.15 0.5] Interaction w/ NPCS
  (Variables|Default|SetDialogueActor (Utilities|Array|Get(acopy) (Class|Actor|GetComponentsbyInterface OtherActor "/Game/Scripts/Dialogue/BP_Interact.BP_Interact_C"))))

(event OnComponentEndOverlap(Sphere)
  (params (OverlappedComponent :type Primitive%20Component%20Object%20Reference) (OtherActor :type Actor%20Object%20Reference) (OtherComp :type Primitive%20Component%20Object%20Reference) (OtherBodyIndex :type Integer))
  ;[0.15 0.15 0.15 0.5] Interaction w/ NPCS
  (Utilities|IsValid (Variables|Default|GetDialogueActor)
    (:Is%20Valid
      (Class|BPInteract|LeaveDialogue(Message) (Variables|Default|GetDialogueActor))
      (Variables|Default|SetDialogueActor 0))))

(event Input|EnhancedActionEvents|EnhancedInputActionIA_Locomotion
  (params (ActionValue :type Float%20%28double-precision%29) (ElapsedSeconds :type Float%20%28double-precision%29) (TriggeredSeconds :type Float%20%28double-precision%29) (InputAction :type Input%20Action%20Object%20Reference :default "/Game/Scripts/Player_Controller/UI/IO/IA_Locomotion.IA_Locomotion"))
  (bind _footsteps_alpha (Variables|Default|GetFootsteps%20Alpha))
  ;[0 0 1 0.5] Basic Movement
  ;;[0 1 0 0.5] Keys: W and S
  (Pawn|Input|AddMovementInput (Transformation|GetActorForwardVector) ActionValue false)
  ;[0.15 0.15 0.15 0.5] Footstep Code
  (if (> (Math|Vector|VectorLength (Transformation|GetVelocity)) 0.0)
    (Audio|Components|Audio|Play _footsteps_alpha)
    (else
      (Audio|Components|Audio|Stop _footsteps_alpha))))

(event Input|EnhancedActionEvents|EnhancedInputActionIA_LookH
  (params (ActionValue :type Float%20%28double-precision%29) (ElapsedSeconds :type Float%20%28double-precision%29) (TriggeredSeconds :type Float%20%28double-precision%29) (InputAction :type Input%20Action%20Object%20Reference :default "/Game/Scripts/Player_Controller/UI/IO/IA_LookH.IA_LookH"))
  ;[0 0 1 0.5] Basic Movement
  ;;[0 1 0 0.5] Look Left and Right
  (Pawn|Input|AddControllerYawInput ActionValue))

(event Input|EnhancedActionEvents|EnhancedInputActionIA_LookV
  (params (ActionValue :type Float%20%28double-precision%29) (ElapsedSeconds :type Float%20%28double-precision%29) (TriggeredSeconds :type Float%20%28double-precision%29) (InputAction :type Input%20Action%20Object%20Reference :default "/Game/Scripts/Player_Controller/UI/IO/IA_LookV.IA_LookV"))
  ;[0 0 1 0.5] Basic Movement
  ;;[0 1 0 0.5] Look Up and Down
  (Pawn|Input|AddControllerPitchInput ActionValue))

(event Input|EnhancedActionEvents|EnhancedInputActionIA_Strafe
  (params (ActionValue :type Float%20%28double-precision%29) (ElapsedSeconds :type Float%20%28double-precision%29) (TriggeredSeconds :type Float%20%28double-precision%29) (InputAction :type Input%20Action%20Object%20Reference :default "/Game/Scripts/Player_Controller/UI/IO/IA_Strafe.IA_Strafe"))
  ;[0 0 1 0.5] Basic Movement
  ;;[0 1 0 0.5] Keys: A and D
  (Pawn|Input|AddMovementInput (Transformation|GetActorRightVector) ActionValue false))

(event Input|EnhancedActionEvents|EnhancedInputActionIA_Journal
  (params (ActionValue :type Boolean) (ElapsedSeconds :type Float%20%28double-precision%29) (TriggeredSeconds :type Float%20%28double-precision%29) (InputAction :type Input%20Action%20Object%20Reference :default "/Game/Scripts/Player_Controller/UI/IO/IA_Journal.IA_Journal"))
  (bind _returnvalue (Game|GetPlayerController 0))
  (bind _journal (Variables|Default|GetJournal))
  ;[1 0.1946 0.4233 0.502] Journal Toggle
  (Utilities|FlowControl|FlipFlop
    (:A
      (Widget|SetVisibility _journal "Visible")
      (Pawn|Components|CharacterMovement|DisableMovement (Variables|Character|GetCharacterMovement))
      (Input|SetInputModeGameandUI _returnvalue 0 "DoNotLock" true false)
      (Variables|/Script/Engine.PlayerController|SetbShowMouseCursor _returnvalue true)
      (Variables|Default|SetJournalUiShowing? _journal))
    (:B
      (Widget|SetVisibility _journal "Hidden")
      (Pawn|Components|CharacterMovement|SetMovementMode (Variables|Character|GetCharacterMovement) "MOVE_Walking" 0)
      (Input|SetInputModeGameandUI _returnvalue 0 "DoNotLock" true false)
      (Variables|/Script/Engine.PlayerController|SetbShowMouseCursor _returnvalue false)
      (Input|SetInputModeGameOnly _returnvalue false))))

(event Input|EnhancedActionEvents|EnhancedInputActionIA_Interact
  (params (ActionValue :type Boolean) (ElapsedSeconds :type Float%20%28double-precision%29) (TriggeredSeconds :type Float%20%28double-precision%29) (InputAction :type Input%20Action%20Object%20Reference :default "/Game/Scripts/Player_Controller/UI/IO/IA_Interact.IA_Interact"))
  (bind _dialogueactor (Variables|Default|GetDialogueActor))
  ;[0.15 0.15 0.15 0.5] Interaction w/ NPCS
  (:Started
    (Utilities|IsValid _dialogueactor
      (:Is%20Valid
        (Class|BPInteract|Interact(Message) _dialogueactor self)))))

(event EventUpdateClues
  (params (Clue%20text :type Text))
  (Default|UpdateClues (Variables|Default|GetJournal) Clue%20text))

(event EventBeginPlay
  ;[1 0 0 0.5] IMC Mapping and Journal Spawn
  (Input|AddMappingContext (PlayerController|LocalPlayerSubsystems|GetEnhancedInputLocalPlayerSubsystem (Game|GetPlayerController 0)) "/Game/Scripts/Player_Controller/UI/IO/IMC_BaseCharacter.IMC_BaseCharacter" 0 "(bIgnoreAllPressedKeysUntilRelease=True,bForceImmediately=False,bNotifyUserSettings=False)")
  (bind _returnvalue (UserInterface|CreateWidget "/Game/UI/Journal/W_Journal.W_Journal_C"))
  (bind _output_get (Variables|Default|SetJournal _returnvalue))
  (UserInterface|Viewport|AddtoViewport _output_get 0)
  (Widget|SetVisibility _output_get "Hidden"))

(event Input|GamepadEvents|GamepadSpecialLeftY
  (params (AxisValue :type Float%20%28single-precision%29))
  (bind _footsteps_alpha (Variables|Default|GetFootsteps%20Alpha))
  ;[0.15 0.15 0.15 0.5] Footstep Code
  (if (> (Math|Vector|VectorLength (Transformation|GetVelocity)) 0.0)
    (Audio|Components|Audio|Play _footsteps_alpha)
    (else
      (Audio|Components|Audio|Stop _footsteps_alpha))))

(event Input|GamepadEvents|GamepadSpecialLeftX
  (params (AxisValue :type Float%20%28single-precision%29))
  (bind _footsteps_alpha (Variables|Default|GetFootsteps%20Alpha))
  ;[0.15 0.15 0.15 0.5] Footstep Code
  (if (> (Math|Vector|VectorLength (Transformation|GetVelocity)) 0.0)
    (Audio|Components|Audio|Play _footsteps_alpha)
    (else
      (Audio|Components|Audio|Stop _footsteps_alpha))))

(event Input|KeyboardEvents|SpaceBar
  (params (Key :type Key%20Structure :default "None"))
  ;[0 0 1 0.5] Basic Movement
  ;;[0 1 0 0.5] Jumping: Space Bar
  (:Pressed
    (Character|Jump))
  (:Released
    (Character|StopJumping)))

(fn ConstructionScript)

(fn FootstepsTrace
  (bind _returnvalue (Transformation|GetActorLocation))
  (bind _capsulecomponent (Variables|Collision|GetCapsuleComponent))
  (bind (_x _y _z) (Math|Vector|BreakVector _returnvalue))
  (bind _returnvalue_2 (Collision|SphereTraceByChannel _returnvalue (Math|Vector|MakeVector _x _y (- _z (Components|Capsule|GetScaledCapsuleHalfHeight _capsulecomponent))) (Components|Capsule|GetScaledCapsuleRadius _capsulecomponent) "TraceTypeQuery1" false 0 "None"))
  (return _returnvalue_2))

(fn TryFootsteps
  (CallFunction|FootstepsTrace)
  (if true
    (Audio|PlaySoundatLocation "/Game/Audio/SoundSFX/woodFootsteps.woodFootsteps" (Transformation|GetActorLocation) "0, 0, 0" 1.0 1.0 0.0 0 0 0 0)))
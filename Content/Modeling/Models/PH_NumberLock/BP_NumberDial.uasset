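; BP_NumberDial is a single rotating digit dial for a number lock puzzle, turned through an arrow widget that receives a reference to the dial.
; RotateDial plays a sound and uses a timeline to yaw the mesh 36 degrees, ignoring input mid-turn.
; When finished, it wraps at 360, derives and prints the digit, then has the parent lock check the turn.
; An optional random-start function exists but is not hooked up.
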(event Custom|FindNumber
  ;[0.4941 1 0.3455] What Number am I on?
  (bind _output_get (Variables|Default|SetNumberNumber (Math|Float|Truncate (/ (Variables|Default|GetNumberDialRotation) 36.0))))
  (Development|PrintString (Utilities|String|ToString(Integer) _output_get)))

(event Custom|RotateDial
  ;[0.212 0.212 0.9045 0.5] Number Dial Can Rotate (And make SFX)
  (if (Variables|Default|GetNumberCanRotate)
    (Variables|Default|SetNumberCanRotate false)
    (Audio|PlaySound2D "/Game/Sound/SFX_LocksTurnDial.SFX_LocksTurnDial" 1.0 1.0 0.0 0 0)
    (bind _alpha (Timeline|NumberDialRotation_TL PlayFromStart)
      (:Update
        (Transformation|SetRelativeRotation (Variables|Default|GetSM_Dial) (Math|Rotator|MakeRotator 0.0 0.0 (+ (Variables|Default|GetNumberDialRotation) (Math|Float|Lerp 0.0 36.0 _alpha))) false false))
      (:Finished
        (Variables|Default|SetNumberDialRotation (+ (Variables|Default|GetNumberDialRotation) (Math|Float|Lerp 0.0 36.0 _alpha)))
        (if (>= (Variables|Default|GetNumberDialRotation) 3.6e+02)
          (Variables|Default|SetNumberDialRotation 0.0)
          (Transformation|SetRelativeRotation (Variables|Default|GetSM_Dial) "0, 0, 0" false false))
        (CallFunction|FindNumber)
        (Default|CheckEveryTurn (Variables|Default|GetNumberLockRef))
        (Variables|Default|SetNumberCanRotate true)))))

(event EventBeginPlay
  ;[1 1 1] Arrows
  (bind _asw_arrow (Utilities|Casting|CastToW_NumberArrow (UserInterface|GetUserWidgetObject (Variables|Default|GetArrow))))
  (Default|NumberInitialize _asw_arrow self))

(fn ConstructionScript)

(fn SetRandomNumber
  ;[1 0.2969 0.9507 0.5] Random Numbers (IF WANTED)
  (bind _output_get (LocalVariables|SetLocalRotation (* (Math|Random|RandomIntegerinRange 0 9) 36.0)))
  (Transformation|SetRelativeRotation (Variables|Default|GetSM_Dial) (Math|Rotator|MakeRotator 0.0 0.0 _output_get) false false)
  (Variables|Default|SetNumberDialRotation (LocalVariables|GetLocalRotation))
  (CallFunction|FindNumber))
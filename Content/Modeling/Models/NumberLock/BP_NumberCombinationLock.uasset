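; BP_NumberCombinationLock is an interactable three-dial combination lock that opens when the dials match its stored code.
; It spawns BP_NumberDial actors onto mesh sockets, passing each a self reference.
; Interacting blends the view to the lock, freezes the player and routes clicks through WidgetInteraction, with Q or Escape exiting.
; CheckEveryTurn compares the dials to the code, and a match plays a sound and timeline, exits the view and destroys lock and dials.
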(event Custom|ExitView
  (bind _returnvalue (Game|GetPlayerCharacter 0))
  (bind _returnvalue_2 (Game|GetPlayerController 0))
  ;[0.2 0.2 1 0.5] Exit the Lock view and Return back to Player
  (Game|Player|SetViewTargetwithBlend _returnvalue_2 _returnvalue 0.5 "VTBlend_Linear" 0.0 false)
  (Input|DisableInput _returnvalue_2)
  (Input|ResetIgnoreLookInput _returnvalue_2)
  (Variables|/Script/Engine.PlayerController|SetbShowMouseCursor _returnvalue_2 false)
  (Pawn|Components|CharacterMovement|SetMovementMode (Variables|/Script/Engine.Character|GetCharacterMovement _returnvalue) "MOVE_Walking" 0)
  (bind _returnvalue_3 (Actor|GetActorOfClass "/Game/Scripts/Player_Controller/BP_GameMode.BP_GameMode_C"))
  (Class|TimeEvent|ReduceTime(Message) _returnvalue_3 1))

(event Custom|CheckEveryTurn
  ;[0.7309 0.7309 0 0.5] Checks Every Dial Rotation to see if you got the Correct Combination, if yes, code below happens
  (bind _number_success (CallFunction|CheckNumberCode))
  (Development|PrintString (Utilities|String|ToString(Boolean) _number_success))
  (if _number_success
    (CallFunction|UnlockNumberLock)))

(event Custom|UnlockNumberLock
  ;[1 0 0 0.5] Correct Combination SFX, leads to Unlocking Animation, then DESTROY
  (Audio|PlaySound2D "/Game/Sound/SFX_LocksUnlock.SFX_LocksUnlock" 1.0 1.0 0.0 0 0)
  (bind _alpha (Timeline|UnlockNumber_TL PlayFromStart)
    (:Update
      (Transformation|SetRelativeLocation (Variables|Default|GetSM_NumberCombinationLock) (Math|Vector|MakeVector 0.0 0.0 (Math|Float|Lerp 0.0 -5.0 _alpha)) false false)
      (Utilities|FlowControl|Delay 1.0)
      (CallFunction|ExitView)
      (Actor|DestroyActor (Variables|Default|GetNumberDials))
      (Actor|DestroyActor))))

(event EventBeginPlay
  ;[0 1 0 0.5] Adds dials to the Number Lock once game begins
  (for _index (range 0 2)
    (bind _returnvalue (Game|SpawnActorfromClass "/Game/Modeling/Models/NumberLock/BP_NumberDial.BP_NumberDial_C" (Math|Transform|MakeTransform "0, 0, 0" "0, 0, 0" "1.000000,1.000000,1.000000") "Undefined" "MultiplyWithRoot" 0 _index self 0))
    (Utilities|Array|Add (Variables|Default|GetNumberDials) _returnvalue)
    (Transformation|AttachComponentToComponent _returnvalue (Variables|Default|GetSM_NumberCombinationLock) (Utilities|Select :Index _index :Option%200 "NumberDial01" :Option%201 "NumberDial02" :Option%202 "NumberDial03") "KeepRelative" "KeepRelative" "KeepRelative" true)))

(event EventInteract
  (params (playerref :type BP%20Detective%20Object%20Reference) (Journal :type W%20Journal%20Object%20Reference))
  (bind _returnvalue (Game|GetPlayerController 0))
  ;[0.2 0.2 1 0.5] Interacted with Lock, so you lose player control and enter Lock View
  (Game|Player|SetViewTargetwithBlend (Game|GetPlayerController 0) self 0.5 "VTBlend_Linear" 0.0 false)
  (Pawn|Components|CharacterMovement|DisableMovement (Variables|/Script/Engine.Character|GetCharacterMovement (Game|GetPlayerCharacter 0)))
  (Input|SetIgnoreLookInput _returnvalue true)
  (Utilities|FlowControl|Delay 0.5)
  (Input|EnableInput _returnvalue)
  (Variables|/Script/Engine.PlayerController|SetbShowMouseCursor _returnvalue true))

(event Input|KeyboardEvents|Q
  (params (Key :type Key%20Structure :default "None"))
  ;[0.5 0 0.5] Q and Esc Inputs to leave Lock View (can be changed)
  (:Pressed
    (CallFunction|ExitView)))

(event Input|KeyboardEvents|Escape
  (params (Key :type Key%20Structure :default "None"))
  ;[0.5 0 0.5] Q and Esc Inputs to leave Lock View (can be changed)
  (:Pressed
    (CallFunction|ExitView)))

(event Input|MouseEvents|LeftMouseButton
  (params (Key :type Key%20Structure :default "None"))
  (bind _widgetinteraction (Variables|Default|GetWidgetInteraction))
  ;[0.731 0.731 0 0.5] Left Mouse Input to Rotate Dial
  (:Pressed
    (Class|WidgetInteractionComponent|PressPointerKey _widgetinteraction "LeftMouseButton"))
  (:Released
    (Class|WidgetInteractionComponent|ReleasePointerKey _widgetinteraction "LeftMouseButton")))

(fn ConstructionScript)

(fn CheckNumberCode
  ;[0.15 0.15 0.15 0.5] Function for Making sure you have the Correct Number Combination
  (bind (_array_element _array_index) (Utilities|Array|ForEachLoopwithBreak (Variables|Default|GetNumberDials) :!label _label)
    (:LoopBody
      (if (== (Variables|/Game/Modeling/Models/NumberLock/BP_NumberDial.BP_NumberDial_C|GetNumberNumber _array_element) (Utilities|Array|Get(acopy) (Variables|Default|GetNumberLockCombination) _array_index))
        (LocalVariables|SetNumberLocalSuccess true)
        (else
          (LocalVariables|SetNumberLocalSuccess false)
          (goto _label Break))))
    (:Completed
      (return (LocalVariables|GetNumberLocalSuccess)))))
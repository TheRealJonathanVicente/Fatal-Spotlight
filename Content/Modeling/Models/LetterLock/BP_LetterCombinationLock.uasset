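; Interactable seven-dial letter combination lock that unlocks its parent drawer or DayLockedDoor.
; Spawns BP_LetterDial actors onto mesh sockets at BeginPlay; interacting blends the view to the lock, freezing the player and enabling a cursor for widget-interaction clicks, with gamepad cursor and exit support.
; CheckEveryTurn compares dials to the combination; a match plays a sound and latch timeline, whose update unlocks the parent, exits the view and destroys the lock.
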(event Custom|UnlockParent
  (bind _parentlockedobject (Variables|Default|GetParentLockedObject))
  (bind _parentlockedobject_2 (Variables|Default|GetParentLockedObject))
  (bind _returnvalue (Actor|GetComponentbyClass _parentlockedobject_2 "/Game/Modeling/Models/Drawers/DrawerBehavior.DrawerBehavior_C"))
  ;[0.15 0.15 0.15 0.5] Unlocking Parent
  (Utilities|IsValid _returnvalue
    (:Is%20Valid
      (Default|Unlock _returnvalue))
    (:Is%20Not%20Valid
      (if (Utilities|ClassIsChildOf (Utilities|GetClass _parentlockedobject) "/Game/Scripts/WorldUpdates/DayLockedDoor.DayLockedDoor_C")
        (Default|Unlock (.AsDay%20Locked%20Door (Utilities|Casting|CastToDayLockedDoor _parentlockedobject)))
        (else
          (Development|PrintString "not a lockable"))))))

(event Custom|ExitView
  (bind _returnvalue (Game|GetPlayerController 0))
  (bind _returnvalue_2 (Game|GetPlayerCharacter 0))
  ;[0.2 0.2 1 0.5] Exit the Lock view and Return back to Player
  (Game|Player|SetViewTargetwithBlend _returnvalue _returnvalue_2 0.5 "VTBlend_Linear" 0.0 false)
  (Input|DisableInput _returnvalue)
  (Input|ResetIgnoreLookInput _returnvalue)
  (Variables|/Script/Engine.PlayerController|SetbShowMouseCursor _returnvalue false)
  (Pawn|Components|CharacterMovement|SetMovementMode (Variables|/Script/Engine.Character|GetCharacterMovement _returnvalue_2) "MOVE_Walking" 0)
  (bind _returnvalue_3 (Actor|GetActorOfClass "/Game/Scripts/Player_Controller/BP_GameMode.BP_GameMode_C"))
  (Class|TimeEvent|ReduceTime(Message) _returnvalue_3 1))

(event Custom|CheckEveryTurn
  ;[0.731 0.731 0 0.5] Checks Every Dial Rotation to see if you got the Correct Combination, if yes, code below happens
  (bind _success (CallFunction|CheckLetterCode))
  (Development|PrintString (Utilities|String|ToString(Boolean) _success))
  (if _success
    (CallFunction|UnlockLetterLock)))

(event Custom|UnlockLetterLock
  ;[1 0 0 0.5] Correct Combination SFX, leads to Unlocking Animation, then DESTROY
  (Audio|PlaySound2D "/Game/Sound/SFX_LocksUnlock.SFX_LocksUnlock" 1.0 1.0 0.0 0 0)
  (bind _alpha (Timeline|UnlockLetter_TL PlayFromStart)
    (:Update
      (Transformation|SetRelativeRotation (Variables|Default|GetSM_LetterLatch) (Math|Rotator|MakeRotator 0.0 (Math|Float|Lerp 0.0 4e+01 _alpha) 0.0) false false)
      (CallFunction|UnlockParent)
      (Utilities|FlowControl|Delay 1.0)
      (CallFunction|ExitView)
      (Actor|DestroyActor (Variables|Default|GetLetterDials))
      (Actor|DestroyActor))))

(event Input|EnhancedActionEvents|EnhancedInputActionIA_Click
  (params (ActionValue :type Boolean) (ElapsedSeconds :type Float%20%28double-precision%29) (TriggeredSeconds :type Float%20%28double-precision%29) (InputAction :type Input%20Action%20Object%20Reference :default "/Game/Scripts/Player_Controller/IO/IA_Click.IA_Click"))
  (bind _widgetinteraction (Variables|Default|GetWidgetInteraction))
  ;[0.731 0.731 0 0.5] Left Mouse Input to Rotate Dial
  (:Triggered
    (Class|WidgetInteractionComponent|PressPointerKey _widgetinteraction "LeftMouseButton"))
  (:Completed
    (Class|WidgetInteractionComponent|ReleasePointerKey _widgetinteraction "LeftMouseButton")))

(event Input|EnhancedActionEvents|EnhancedInputActionIA_MenuMoveCorsor
  (params (ActionValue :type Vector%202D%20Structure) (ElapsedSeconds :type Float%20%28double-precision%29) (TriggeredSeconds :type Float%20%28double-precision%29) (InputAction :type Input%20Action%20Object%20Reference :default "/Game/Scripts/Player_Controller/IO/IA_MenuMoveCorsor.IA_MenuMoveCorsor"))
  (bind _returnvalue (Game|GetPlayerController 0))
  (bind (_locationx _locationy) (Game|Player|GetMousePosition _returnvalue))
  (if (Variables|/Script/Engine.PlayerController|GetbShowMouseCursor (Game|GetPlayerController 0))
    (Class|PlayerController|SetMouseLocation (Game|GetPlayerController 0) (Math|Float|Round (+ (* (.x ActionValue) 15.0) _locationx)) (Math|Float|Round (+ (* (.y ActionValue) -15.0) _locationy)))))

(event EventBeginPlay
  ;[0 1 0 0.5] Adds Dials to the Letter Lock once the game begins
  (for _index (range 0 6)
    (bind _returnvalue (Game|SpawnActorfromClass "/Game/Modeling/Models/LetterLock/BP_LetterDial.BP_LetterDial_C" (Math|Transform|MakeTransform "0, 0, 0" "0, 0, 0" "1.000000,1.000000,1.000000") "Undefined" "MultiplyWithRoot" 0 _index self 0))
    (Utilities|Array|Add (Variables|Default|GetLetterDials) _returnvalue)
    (Transformation|AttachComponentToComponent _returnvalue (Variables|Default|GetSM_LetterCombinationLock) (Utilities|Select :Index _index :Option%200 "LetterDial01" :Option%201 "LetterDial02" :Option%202 "LetterDial03" :Option%203 "LetterDial04" :Option%204 "LetterDial05" :Option%205 "LetterDial06" :Option%206 "LetterDial07") "KeepRelative" "KeepRelative" "KeepRelative" true)))

(event EventInteract
  (params (playerref :type BP%20Detective%20Object%20Reference) (Journal :type W%20Journal%20Object%20Reference))
  (bind _returnvalue (Game|GetPlayerController 0))
  ;[0.2 0.2 1 0.5] Interacted with Lock, so you lose player control and enter Lock View
  (Game|Player|SetViewTargetwithBlend (Game|GetPlayerController 0) self 0.5 "VTBlend_Linear" 0.0 false)
  (Pawn|Components|CharacterMovement|DisableMovement (Variables|/Script/Engine.Character|GetCharacterMovement (Game|GetPlayerCharacter 0)))
  (Input|SetIgnoreLookInput _returnvalue true)
  (Utilities|FlowControl|Delay 0.5)
  (Input|EnableInput _returnvalue)
  (Variables|/Script/Engine.PlayerController|SetbShowMouseCursor _returnvalue true))

(event Input|GamepadEvents|GamepadFaceButtonRight
  (params (Key :type Key%20Structure :default "None"))
  ;[0.5 0 0.5] Q and Esc Inputs to leave Lock View (can be changed)
  (:Pressed
    (CallFunction|ExitView)))

(event Input|MouseEvents|LeftMouseButton
  (params (Key :type Key%20Structure :default "None"))
  (bind _widgetinteraction (Variables|Default|GetWidgetInteraction))
  ;[0.731 0.731 0 0.5] Left Mouse Input to Rotate Dial
  (:Pressed
    (Class|WidgetInteractionComponent|PressPointerKey _widgetinteraction "LeftMouseButton"))
  (:Released
    (Class|WidgetInteractionComponent|ReleasePointerKey _widgetinteraction "LeftMouseButton")))

(event Input|KeyboardEvents|Escape
  (params (Key :type Key%20Structure :default "None"))
  ;[0.5 0 0.5] Q and Esc Inputs to leave Lock View (can be changed)
  (:Pressed
    (CallFunction|ExitView)))

(event Input|KeyboardEvents|Q
  (params (Key :type Key%20Structure :default "None"))
  ;[0.5 0 0.5] Q and Esc Inputs to leave Lock View (can be changed)
  (:Pressed
    (CallFunction|ExitView)))

(fn ConstructionScript)

(fn CheckLetterCode
  ;[0.15 0.15 0.15 0.5] Function for Making sure you have the Correct Letter Combination
  (bind (_array_element _array_index) (Utilities|Array|ForEachLoopwithBreak (Variables|Default|GetLetterDials) :!label _label)
    (:LoopBody
      (if (== (Variables|/Game/Modeling/Models/LetterLock/BP_LetterDial.BP_LetterDial_C|GetLetterNumber _array_element) (Utilities|Array|Get(acopy) (Variables|Default|GetLetterLockCombination) _array_index))
        (LocalVariables|SetLetterLocalSuccess true)
        (else
          (LocalVariables|SetLetterLocalSuccess false)
          (goto _label Break))))
    (:Completed
      (return (LocalVariables|GetLetterLocalSuccess)))))
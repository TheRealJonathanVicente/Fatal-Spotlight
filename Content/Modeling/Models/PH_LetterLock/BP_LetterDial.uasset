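; BP_LetterDial is a single rotating dial of a letter lock puzzle, with an arrow widget that receives a reference to it on BeginPlay.
; RotateDial plays a sound and a timeline that rolls the mesh one of sixteen steps, blocking input until finished and resetting after a full turn.
; Each turn derives the letter index from the rotation, then has the owning lock check the combination.
; An optional random-start function exists but is unused.
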(event Custom|RotateDial
  ;[0.212 0.212 0.9045 0.5] Number Dial Can Rotate (And make SFX)
  (if (Variables|Default|GetLetterCanRotate)
    (Variables|Default|SetLetterCanRotate false)
    (Audio|PlaySound2D "/Game/Sound/SFX_LocksTurnDial.SFX_LocksTurnDial" 1.0 1.0 0.0 0 0)
    (bind _alpha (Timeline|LetterDialRotaton_TL PlayFromStart)
      (:Update
        (Transformation|SetRelativeRotation (Variables|Default|GetSM_LetterDial) (Math|Rotator|MakeRotator (+ (Variables|Default|GetLetterDialRotation) (Math|Float|Lerp 0.0 22.5 _alpha)) 0.0 0.0) false false))
      (:Finished
        (Variables|Default|SetLetterDialRotation (+ (Variables|Default|GetLetterDialRotation) (Math|Float|Lerp 0.0 22.5 _alpha)))
        (if (>= (Variables|Default|GetLetterDialRotation) 3.6e+02)
          (Variables|Default|SetLetterDialRotation 0.0)
          (Transformation|SetRelativeRotation (Variables|Default|GetSM_LetterDial) "0, 0, 0" false false))
        (CallFunction|FindLetter)
        (Default|CheckEveryTurn (Variables|Default|GetLetterLockRef))
        (Variables|Default|SetLetterCanRotate true)))))

(event Custom|FindLetter
  ;[0.4941 1 0.3455] What Number am I on?
  (bind _output_get (Variables|Default|SetLetterNumber (Math|Float|Truncate (/ (Variables|Default|GetLetterDialRotation) 22.5))))
  (Development|PrintString (Utilities|String|ToString(Integer) _output_get)))

(event EventBeginPlay
  ;[1 1 1] Arrows
  (bind _asw_letter_arrow (Utilities|Casting|CastToW_LetterArrow (UserInterface|GetUserWidgetObject (Variables|Default|GetArrow))))
  (Default|LetterInitialize _asw_letter_arrow self))

(fn ConstructionScript)

(fn SetRandomLetter
  ;[1 0.2969 0.9507 0.5] Random Letters (IF WANTED)
  (bind _output_get (LocalVariables|SetLocalRotation (* (Math|Random|RandomIntegerinRange 0 15) 22.5)))
  (Transformation|SetRelativeRotation (Variables|Default|GetSM_LetterDial) (Math|Rotator|MakeRotator _output_get 0.0 0.0) false false)
  (Variables|Default|SetLetterDialRotation (LocalVariables|GetLocalRotation))
  (CallFunction|FindLetter))
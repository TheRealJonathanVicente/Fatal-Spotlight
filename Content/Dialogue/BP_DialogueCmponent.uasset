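; Dialogue component that shows and advances a conversation, one line each time Interact is called.
; The first call creates a WB_Dialogue widget with the speaker's name, and later calls update its text.
; Lines form a data-driven chain: each data table row names the next row and table, so conversations can cross tables.
; A row's EndDialogue flag makes the following Interact remove and clear the widget.
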(event EventBeginPlay)

(event EventTick
  (params (DeltaSeconds :type Float%20%28single-precision%29)))

(event EventInteract
  (params (playerref :type BP%20Detective%20Object%20Reference))
  (if (Variables|Default|GetEndDialogue)
    (Widget|RemovefromParent (Variables|Default|GetDialogueWidget))
    (Variables|Default|SetEndDialogue false)
    (Variables|Default|SetDialogueWidget 0)
    (else
      (Utilities|IsValid (Variables|Default|GetDialogueWidget)
        (:Is%20Valid
          (bind _returnvalue (Utilities|GetDataTableRow (Variables|Default|GetData%20Table) (Variables|Default|GetRow%20Name))
            (:then
              (Default|UpdateDialogue (Variables|Default|GetDialogueWidget) (.Dialogue (Utilities|Struct|BreakDialogue_Sructure _returnvalue)))
              (Variables|Default|SetRow%20Name (.Row (Utilities|Struct|BreakDialogue_Sructure _returnvalue)))
              (Variables|Default|SetData%20Table (.DataTable (Utilities|Struct|BreakDialogue_Sructure _returnvalue)))
              (Variables|Default|SetEndDialogue (.EndDialogue? (Utilities|Struct|BreakDialogue_Sructure _returnvalue))))))
        (:Is%20Not%20Valid
          (bind _returnvalue_2 (Utilities|GetDataTableRow (Variables|Default|GetData%20Table) (Variables|Default|GetRow%20Name))
            (:then
              (bind _returnvalue_3 (UserInterface|CreateWidget "/Game/Dialogue/WB_Dialogue.WB_Dialogue_C" 0 (Utilities|Text|ToText(Name) (Variables|Default|GetName)) (.Dialogue (Utilities|Struct|BreakDialogue_Sructure _returnvalue_2))))
              (bind _output_get (Variables|Default|SetDialogueWidget _returnvalue_3))
              (UserInterface|Viewport|AddtoViewport _output_get 0)
              (Variables|Default|SetRow%20Name (.Row (Utilities|Struct|BreakDialogue_Sructure _returnvalue_2)))
              (Variables|Default|SetData%20Table (.DataTable (Utilities|Struct|BreakDialogue_Sructure _returnvalue_2)))
              (Variables|Default|SetEndDialogue (.EndDialogue? (Utilities|Struct|BreakDialogue_Sructure _returnvalue_2))))))))))
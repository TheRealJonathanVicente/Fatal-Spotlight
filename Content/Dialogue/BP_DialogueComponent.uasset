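; Dialogue component that runs branching, data-table-driven conversations in an on-screen widget.
; Interact opens or advances the dialogue, each row supplying the next row, table and end flag.
; Open-ended rows spawn option widgets on opening or after OptionSelected, but not when Interact advances an open dialogue.
; Ending or leaving removes the widget, restores game-only input and calls ReduceTime on BP_GameMode.
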(event Custom|OptionSelected
  (params (RowName :type Name) (DataTable :type Data%20Table%20Object%20Reference))
  (bind _returnvalue (Game|GetPlayerController 0))
  (bind _returnvalue_2 (Utilities|GetDataTableRow DataTable RowName)
    (:then
      (Widget|Panel|ClearChildren (Variables|/Game/Dialogue/WB_Dialogue.WB_Dialogue_C|GetOptionScrollBox (Variables|Default|GetDialogueWidget)))
      (Default|UpdateDialogue (Variables|Default|GetDialogueWidget) (.Dialogue (Utilities|Struct|BreakDialogue_Sructure _returnvalue_2)))
      (Variables|Default|SetRow%20Name (.Row (Utilities|Struct|BreakDialogue_Sructure _returnvalue_2)))
      (Variables|Default|SetData%20Table (.DataTable (Utilities|Struct|BreakDialogue_Sructure _returnvalue_2)))
      (Variables|Default|SetEndDialogue (.EndDialogue? (Utilities|Struct|BreakDialogue_Sructure _returnvalue_2)))
      (Input|SetInputModeGameandUI _returnvalue 0 "DoNotLock" true false)
      (Variables|/Script/Engine.PlayerController|SetbShowMouseCursor _returnvalue true)
      (if (.OpenEndedDialogue? (Utilities|Struct|BreakDialogue_Sructure _returnvalue_2))
        (for _array_element (.OpenEndedDialogueOptions (Utilities|Struct|BreakDialogue_Sructure _returnvalue_2))
          (bind _returnvalue_3 (UserInterface|CreateWidget "/Game/Dialogue/WB_Options.WB_Options_C" 0 (Utilities|Text|ToText(Name) (.OptionName (Utilities|Struct|BreakOptionsDialogue_Structure _array_element))) self (.Row (Utilities|Struct|BreakOptionsDialogue_Structure _array_element)) (.DataTable (Utilities|Struct|BreakOptionsDialogue_Structure _array_element)) (.IsLeave (Utilities|Struct|BreakOptionsDialogue_Structure _array_element))))
          (Widget|Panel|AddChild (Variables|/Game/Dialogue/WB_Dialogue.WB_Dialogue_C|GetOptionScrollBox (Variables|Default|GetDialogueWidget)) _returnvalue_3))))))

(event EventBeginPlay)

(event EventTick
  (params (DeltaSeconds :type Float%20%28single-precision%29)))

(event EventInteract
  (params (playerref :type BP%20Detective%20Object%20Reference))
  (bind _returnvalue (Game|GetPlayerController 0))
  (bind _returnvalue_2 (Game|GetPlayerController 0))
  (if (Variables|Default|GetEndDialogue)
    (Widget|RemovefromParent (Variables|Default|GetDialogueWidget))
    (Variables|Default|SetEndDialogue false)
    (Variables|Default|SetDialogueWidget 0)
    (Input|SetInputModeGameandUI _returnvalue_2 0 "DoNotLock" true false)
    (Variables|/Script/Engine.PlayerController|SetbShowMouseCursor _returnvalue_2 false)
    (Input|SetInputModeGameOnly _returnvalue_2 false)
    (bind _returnvalue_3 (Actor|GetActorOfClass "/Game/Player_Controller/BP_GameMode.BP_GameMode_C"))
    (Default|ReduceTime _returnvalue_3 false)
    (else
      (Utilities|IsValid (Variables|Default|GetDialogueWidget)
        (:Is%20Valid
          (bind _returnvalue_4 (Utilities|GetDataTableRow (Variables|Default|GetData%20Table) (Variables|Default|GetRow%20Name))
            (:then
              (Default|UpdateDialogue (Variables|Default|GetDialogueWidget) (.Dialogue (Utilities|Struct|BreakDialogue_Sructure _returnvalue_4)))
              (Variables|Default|SetRow%20Name (.Row (Utilities|Struct|BreakDialogue_Sructure _returnvalue_4)))
              (Variables|Default|SetData%20Table (.DataTable (Utilities|Struct|BreakDialogue_Sructure _returnvalue_4)))
              (Variables|Default|SetEndDialogue (.EndDialogue? (Utilities|Struct|BreakDialogue_Sructure _returnvalue_4))))))
        (:Is%20Not%20Valid
          (bind _returnvalue_5 (Utilities|GetDataTableRow (Variables|Default|GetData%20Table) (Variables|Default|GetRow%20Name))
            (:then
              (bind _returnvalue_6 (UserInterface|CreateWidget "/Game/Dialogue/WB_Dialogue.WB_Dialogue_C" 0 (Utilities|Text|ToText(Name) (Variables|Default|GetName)) (.Dialogue (Utilities|Struct|BreakDialogue_Sructure _returnvalue_5))))
              (bind _output_get (Variables|Default|SetDialogueWidget _returnvalue_6))
              (UserInterface|Viewport|AddtoViewport _output_get 0)
              (Variables|Default|SetRow%20Name (.Row (Utilities|Struct|BreakDialogue_Sructure _returnvalue_5)))
              (Variables|Default|SetData%20Table (.DataTable (Utilities|Struct|BreakDialogue_Sructure _returnvalue_5)))
              (Variables|Default|SetEndDialogue (.EndDialogue? (Utilities|Struct|BreakDialogue_Sructure _returnvalue_5)))
              (Input|SetInputModeGameandUI _returnvalue 0 "DoNotLock" true false)
              (Variables|/Script/Engine.PlayerController|SetbShowMouseCursor _returnvalue true)
              (if (.OpenEndedDialogue? (Utilities|Struct|BreakDialogue_Sructure _returnvalue_5))
                (for _array_element (.OpenEndedDialogueOptions (Utilities|Struct|BreakDialogue_Sructure _returnvalue_5))
                  (bind _returnvalue_7 (UserInterface|CreateWidget "/Game/Dialogue/WB_Options.WB_Options_C" 0 (Utilities|Text|ToText(Name) (.OptionName (Utilities|Struct|BreakOptionsDialogue_Structure _array_element))) self (.Row (Utilities|Struct|BreakOptionsDialogue_Structure _array_element)) (.DataTable (Utilities|Struct|BreakOptionsDialogue_Structure _array_element)) (.IsLeave (Utilities|Struct|BreakOptionsDialogue_Structure _array_element))))
                  (Widget|Panel|AddChild (Variables|/Game/Dialogue/WB_Dialogue.WB_Dialogue_C|GetOptionScrollBox (Variables|Default|GetDialogueWidget)) _returnvalue_7))))))))))

(event EventLeaveDialogue
  (bind _returnvalue (Game|GetPlayerController 0))
  (Utilities|IsValid (Variables|Default|GetDialogueWidget)
    (:Is%20Valid
      (Widget|RemovefromParent (Variables|Default|GetDialogueWidget))
      (Variables|Default|SetEndDialogue false)
      (Variables|Default|SetDialogueWidget 0)
      (Input|SetInputModeGameandUI _returnvalue 0 "DoNotLock" true false)
      (Variables|/Script/Engine.PlayerController|SetbShowMouseCursor _returnvalue false)
      (Input|SetInputModeGameOnly _returnvalue false)
      (bind _returnvalue_2 (Actor|GetActorOfClass "/Game/Player_Controller/BP_GameMode.BP_GameMode_C"))
      (Default|ReduceTime _returnvalue_2 false))))
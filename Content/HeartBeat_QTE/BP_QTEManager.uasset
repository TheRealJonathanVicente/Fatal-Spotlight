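; BP_QTEManager runs a heartbeat quick-time event where a press must be registered before each countdown expires.
; Each beat resets the countdown from HeartbeatInterval and starts a looping timer that decrements it, failing the QTE at zero.
; A valid press clears TimerHadle and starts the next beat after a short delay, though the graph never assigns that handle.
; Feedback is debug text only, with no success end state.
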(event Custom|StartHeartbeatQTE
  ;[0.15 0.15 0.15 0.5] StartHeartbeatQTE
  (Variables|Default|SetIsInQTE true)
  (Variables|Default|SetFailed false)
  (CallFunction|NextHeartbeat))

(event Custom|NextHeartbeat
  ;[0.15 0.15 0.15 0.5] NextHeartbeat
  (Variables|Default|SetCurrentTime (Variables|Default|GetHeartbeatInterval))
  (Utilities|Time|SetTimerbyEvent (delegate Custom|TickHeartbeat) 0.1 true))

(event Custom|TickHeartbeat
  ;[0.15 0.15 0.15 0.5] TickHeartbeat
  (Variables|Default|SetCurrentTime (- (Variables|Default|GetCurrentTime) 0.1))
  (if (<= (Variables|Default|GetCurrentTime) 0.0)
    (CallFunction|FailedHeartbeat)))

(event Custom|FailedHeartbeat
  ;[0.15 0.15 0.15 0.5] Failed!
  (Variables|Default|SetFailed true)
  (Variables|Default|SetIsInQTE false)
  (Development|PrintText "Failed!"))

(event Custom|RegisterHeartbeatPress
  ;[0.15 0.15 0.15 0.5] Register a Press
  (if (and (Variables|Default|GetIsInQTE) (not (Variables|Default|GetFailed)))
    (Utilities|Time|ClearandInvalidateTimerbyHandle (Variables|Default|GetTimerHadle))
    (Development|PrintString "Good Press")
    (Utilities|FlowControl|Delay 0.2)
    (CallFunction|NextHeartbeat)))

(event Collision|EventActorBeginOverlap
  (params (OtherActor :type Actor%20Object%20Reference)))

(event EventTick
  (params (DeltaSeconds :type Float%20%28single-precision%29)))

(fn ConstructionScript)
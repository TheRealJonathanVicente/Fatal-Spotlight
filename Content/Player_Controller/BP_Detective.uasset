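; BP_Detective is the player character for a detective game, with Enhanced Input movement and look, jumping, and a HUD widget.
; Pressing E line-traces forward from the capsule to interact with clues through BPI_Interact.
; A sphere overlap stores the nearby dialogue component for IA_Interact and ends dialogue on exit.
; A looping timer runs a zero-length trace whose result is unused, and the sphere-trace focus logic is disconnected.
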(event OnComponentBeginOverlap(Sphere)
  (params (OverlappedComponent :type Primitive%20Component%20Object%20Reference) (OtherActor :type Actor%20Object%20Reference) (OtherComp :type Primitive%20Component%20Object%20Reference) (OtherBodyIndex :type Integer) (bFromSweep :type Boolean) (SweepResult :type Hit%20Result%20Structure%20%28by%20ref%29))
  ;[0.15 0.15 0.15 0.5] Interaction w/ NPCS
  (Variables|Default|SetDialogueActor (Utilities|Array|Get(acopy) (Class|Actor|GetComponentsbyInterface OtherActor "/Game/Dialogue/BPI_Interact.BPI_Interact_C"))))

(event OnComponentEndOverlap(Sphere)
  (params (OverlappedComponent :type Primitive%20Component%20Object%20Reference) (OtherActor :type Actor%20Object%20Reference) (OtherComp :type Primitive%20Component%20Object%20Reference) (OtherBodyIndex :type Integer))
  ;[0.15 0.15 0.15 0.5] Interaction w/ NPCS
  (Utilities|IsValid (Variables|Default|GetDialogueActor)
    (:Is%20Valid
      (Class|BPIInteract|LeaveDialogue(Message) (Variables|Default|GetDialogueActor))
      (Variables|Default|SetDialogueActor 0))))

(event Custom|Create%20Interaction%20Trace
  ;[0.15 0.15 0.15 0.5] Clue Interaction JV
  (CallFunction|ClueInteraction 0.0))

(event Input|EnhancedActionEvents|EnhancedInputActionIA_Locomotion
  (params (ActionValue :type Float%20%28double-precision%29) (ElapsedSeconds :type Float%20%28double-precision%29) (TriggeredSeconds :type Float%20%28double-precision%29) (InputAction :type Input%20Action%20Object%20Reference :default "/Game/Player_Controller/UI/IO/IA_Locomotion.IA_Locomotion"))
  ;[0 0 1 0.5] Basic Movement
  ;;[0 1 0 0.5] Keys: W and S
  (Pawn|Input|AddMovementInput (Transformation|GetActorForwardVector) ActionValue false))

(event Input|EnhancedActionEvents|EnhancedInputActionIA_LookH
  (params (ActionValue :type Float%20%28double-precision%29) (ElapsedSeconds :type Float%20%28double-precision%29) (TriggeredSeconds :type Float%20%28double-precision%29) (InputAction :type Input%20Action%20Object%20Reference :default "/Game/Player_Controller/UI/IO/IA_LookH.IA_LookH"))
  ;[0 0 1 0.5] Basic Movement
  ;;[0 1 0 0.5] Look Left and Right
  (Pawn|Input|AddControllerYawInput ActionValue))

(event Input|EnhancedActionEvents|EnhancedInputActionIA_LookV
  (params (ActionValue :type Float%20%28double-precision%29) (ElapsedSeconds :type Float%20%28double-precision%29) (TriggeredSeconds :type Float%20%28double-precision%29) (InputAction :type Input%20Action%20Object%20Reference :default "/Game/Player_Controller/UI/IO/IA_LookV.IA_LookV"))
  ;[0 0 1 0.5] Basic Movement
  ;;[0 1 0 0.5] Look Up and Down
  (Pawn|Input|AddControllerPitchInput ActionValue))

(event Input|EnhancedActionEvents|EnhancedInputActionIA_Strafe
  (params (ActionValue :type Float%20%28double-precision%29) (ElapsedSeconds :type Float%20%28double-precision%29) (TriggeredSeconds :type Float%20%28double-precision%29) (InputAction :type Input%20Action%20Object%20Reference :default "/Game/Player_Controller/UI/IO/IA_Strafe.IA_Strafe"))
  ;[0 0 1 0.5] Basic Movement
  ;;[0 1 0 0.5] Keys: A and D
  (Pawn|Input|AddMovementInput (Transformation|GetActorRightVector) ActionValue false))

(event Input|EnhancedActionEvents|EnhancedInputActionIA_Interact
  (params (ActionValue :type Boolean) (ElapsedSeconds :type Float%20%28double-precision%29) (TriggeredSeconds :type Float%20%28double-precision%29) (InputAction :type Input%20Action%20Object%20Reference :default "/Game/Player_Controller/UI/IO/IA_Interact.IA_Interact"))
  (bind _dialogueactor (Variables|Default|GetDialogueActor))
  ;[0.15 0.15 0.15 0.5] Interaction w/ NPCS
  (:Started
    (Utilities|IsValid _dialogueactor
      (:Is%20Valid
        (Class|BPIInteract|Interact(Message) _dialogueactor self)))))

(event EventBeginPlay
  ;[1 0 0 0.5] IMC Mapping
  (Utilities|FlowControl|Sequence
    (:then_0
      (Input|AddMappingContext (PlayerController|LocalPlayerSubsystems|GetEnhancedInputLocalPlayerSubsystem (Game|GetPlayerController 0)) "/Game/Player_Controller/UI/IO/IMC_BaseCharacter.IMC_BaseCharacter" 0 "(bIgnoreAllPressedKeysUntilRelease=True,bForceImmediately=False,bNotifyUserSettings=False)"))
    (:then_1
      ;[0.15 0.15 0.15 0.5] Clue Interaction JV
      (bind _returnvalue (Utilities|Time|SetTimerbyFunctionName 0 "Create Interaction Trace" 0.01 true))
      (Variables|Default|SetInteractionTimer _returnvalue)
      (bind _returnvalue_2 (UserInterface|CreateWidget "/Game/UI_HUD.UI_HUD_C"))
      (UserInterface|Viewport|AddtoViewport _returnvalue_2 0))))

(event Input|KeyboardEvents|E
  (params (Key :type Key%20Structure :default "None"))
  ;[0.15 0.15 0.15 0.5] Clue Interaction JV
  (:Pressed
    (bind _hitactor (CallFunction|ClueInteraction 3.5e+02))
    (if (and (Utilities|IsValid _hitactor) (Utilities|DoesObjectImplementInterface _hitactor "/Game/Dialogue/BPI_Interact.BPI_Interact_C"))
      (Class|BPIInteract|Interact(Message) _hitactor))))

(event Input|KeyboardEvents|SpaceBar
  (params (Key :type Key%20Structure :default "None"))
  ;[0 0 1 0.5] Basic Movement
  ;;[0 1 0 0.5] Jumping: Space Bar
  (:Pressed
    (Character|Jump))
  (:Released
    (Character|StopJumping)))

(fn ConstructionScript)

(fn ClueInteraction
  (params (Length :type Float%20%28double-precision%29))
  (bind _capsulecomponent (Variables|Collision|GetCapsuleComponent))
  (bind _returnvalue (Transformation|GetWorldLocation _capsulecomponent))
  (bind _outhit (Collision|LineTraceByChannel _returnvalue (+ (* (Math|Vector|GetForwardVector _capsulecomponent) Length) _returnvalue) "TraceTypeQuery1" false 0 "None"))
  (return (.HitActor (Collision|BreakHitResult _outhit))))
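; BP_MasterClue is a clue actor that shows an interaction prompt when BP_Detective comes within range.
; While CanInteract is set, sphere overlap creates a UI_Interact widget, animates it in, applies an outline overlay material and sets CanPressE.
; Leaving reverses the animation, clears the outline and removes the widget after a short delay.
; The trace event and IA_Interact input only print debug strings.
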(event OnComponentBeginOverlap(Sphere)
  (params (OverlappedComponent :type Primitive%20Component%20Object%20Reference) (OtherActor :type Actor%20Object%20Reference) (OtherComp :type Primitive%20Component%20Object%20Reference) (OtherBodyIndex :type Integer) (bFromSweep :type Boolean) (SweepResult :type Hit%20Result%20Structure%20%28by%20ref%29))
  ;[0.15 0.15 0.15 0.5] Sphere Collision (Inside)
  (Utilities|Casting|CastToBP_Detective OtherActor)
  (if (Variables|Default|GetCanInteract)
    (bind _returnvalue (UserInterface|CreateWidget "/Game/UI_Interact.UI_Interact_C"))
    (bind _output_get (Variables|Default|SetInteraction%20Widget _returnvalue))
    (UserInterface|SetWidget (Variables|Default|GetWidget) _output_get)
    (Rendering|SetVisibility (Variables|Default|GetWidget) true false)
    (bind _interaction_widget (Variables|Default|GetInteraction%20Widget)
      (:then
        (if (not (Variables|Default|GetHintVisible))
          (UserInterface|Animation|PlayAnimation _interaction_widget 0 0.0 1 "Forward" 1.5 false)
          (Variables|Default|SetHintVisible true)
          (Rendering|Material|SetOverlayMaterial (Variables|Default|GetStaticMesh) "/Game/M_Outline.M_Outline" :!class /Script/Engine.MeshComponent)
          (Variables|Default|SetCanPressE true)))
      (:else))))

(event OnComponentEndOverlap(Sphere)
  (params (OverlappedComponent :type Primitive%20Component%20Object%20Reference) (OtherActor :type Actor%20Object%20Reference) (OtherComp :type Primitive%20Component%20Object%20Reference) (OtherBodyIndex :type Integer))
  ;[0.15 0.15 0.15 0.5] Sphere Collision (Outside)
  (Utilities|Casting|CastToBP_Detective OtherActor)
  (if (Variables|Default|GetCanInteract)
    (bind _interaction_widget (Variables|Default|GetInteraction%20Widget)
      (:then
        (if (Variables|Default|GetHintVisible)
          (UserInterface|Animation|PlayAnimation _interaction_widget 0 0.0 1 "Reverse" 1.5 false)
          (Variables|Default|SetHintVisible false)
          (Variables|Default|SetCanPressE false)
          (Rendering|Material|SetOverlayMaterial (Variables|Default|GetStaticMesh) 0 :!class /Script/Engine.MeshComponent))
        (Utilities|FlowControl|Delay 0.15)
        (Widget|RemovefromParent (Variables|Default|GetInteraction%20Widget))
        (Variables|Default|SetInteraction%20Widget 0)
        (Rendering|SetVisibility (Variables|Default|GetWidget) false false))
      (:else))))

(event Custom|Can%20Recieve%20Trace_1
  (params (CanInteract :type Boolean))
  (if (Variables|Default|GetCanInteract)
    (if CanInteract
      (Development|PrintString "tEST 5"))))

(event Input|EnhancedActionEvents|EnhancedInputActionIA_Interact
  (params (ActionValue :type Boolean) (ElapsedSeconds :type Float%20%28double-precision%29) (TriggeredSeconds :type Float%20%28double-precision%29) (InputAction :type Input%20Action%20Object%20Reference :default "/Game/Scripts/Player_Controller/IO/IA_Interact.IA_Interact"))
  (Development|PrintString "Test 69"))

(event EventBeginPlay)

(event Collision|EventActorBeginOverlap
  (params (OtherActor :type Actor%20Object%20Reference)))

(event EventTick
  (params (DeltaSeconds :type Float%20%28single-precision%29)))

(fn ConstructionScript)